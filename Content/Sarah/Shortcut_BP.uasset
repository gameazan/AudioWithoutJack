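; Shortcut actor that reveals and animates a row of letter meshes, apparently spelling "SHORTCUT", one after another when its move event fires.
; The event speeds up eight timelines, then chains them so each starts when the previous finishes.
; Each timeline feeds its scaled track into the Down function, which makes that letter visible and sets its relative Z, leaving X and Y unchanged.
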(event Custom|move
  (for _array_element (Utilities|Array|MakeArray (Variables|Default|GetTimeline) (Variables|Default|GetTimeline_6) (Variables|Default|GetTimeline_5) (Variables|Default|GetTimeline_4) (Variables|Default|GetTimeline_3) (Variables|Default|GetTimeline_2) (Variables|Default|GetTimeline_1) (Variables|Default|GetTimeline_0))
    (Components|Timeline|SetPlayRate _array_element 6.5))
  (bind _newtrack_0 (Timeline|Timeline Play)
    (:Update
      (CallFunction|Down (Variables|Default|Gets) (* _newtrack_0 1e+03)))
    (:Finished
      (bind _newtrack_0_2 (Timeline|Timeline_0 Play)
        (:Update
          (CallFunction|Down (Variables|Default|Geth) (* _newtrack_0_2 1e+03)))
        (:Finished
          (bind _newtrack_0_3 (Timeline|Timeline_1 Play)
            (:Update
              (CallFunction|Down (Variables|Default|Geto) (* _newtrack_0_3 1e+03)))
            (:Finished
              (bind _newtrack_0_4 (Timeline|Timeline_2 Play)
                (:Update
                  (CallFunction|Down (Variables|Default|Getr) (* _newtrack_0_4 1e+03)))
                (:Finished
                  (bind _newtrack_0_5 (Timeline|Timeline_3 Play)
                    (:Update
                      (CallFunction|Down (Variables|Default|Gett) (* _newtrack_0_5 1e+03)))
                    (:Finished
                      (bind _newtrack_0_6 (Timeline|Timeline_4 Play)
                        (:Update
                          (CallFunction|Down (Variables|Default|Getc) (* _newtrack_0_6 1e+03)))
                        (:Finished
                          (bind _newtrack_0_7 (Timeline|Timeline_5 Play)
                            (:Update
                              (CallFunction|Down (Variables|Default|Getu) (* _newtrack_0_7 1e+03)))
                            (:Finished
                              (bind _newtrack_0_8 (Timeline|Timeline_6 Play)
                                (:Update
                                  (CallFunction|Down (Variables|Default|Getu1) (* _newtrack_0_8 1e+03)))))))))))))))))))

(event EventBeginPlay)

(event Collision|EventActorBeginOverlap
  (params (OtherActor :type Actor%20Object%20Reference)))

(event EventTick
  (params (DeltaSeconds :type Float%20%28single-precision%29)))

(fn ConstructionScript)

(fn Down
  (params (mesh :type Static%20Mesh%20Component%20Object%20Reference) (alpha :type Float%20%28double-precision%29))
  (bind _relativelocation (Variables|/Script/Engine.SceneComponent|GetRelativeLocation mesh))
  (Rendering|SetVisibility mesh true false)
  (Transformation|SetRelativeLocation mesh (Math|Vector|MakeVector (.x _relativelocation) (.y _relativelocation) alpha) false false))