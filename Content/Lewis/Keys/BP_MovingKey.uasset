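; Moving keyboard key actor that, while ShouldMove is set, waits a random time then slides one step along X or Y.
; When the timer expires, CalculateMovement sphere-traces four directions on the KeyboardKey profile and Tick picks randomly among the unblocked ones.
; Move eases toward that offset with VInterpTo every frame; nothing here clears IsMoving, so the cycle never restarts.
; Debug prints and persistent trace drawing are left in.
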(event EventBeginPlay
  (CallFunction|SetMoveTimer)
  (Variables|Default|SetMoveTimer (Variables|Default|GetTimeBetweenMoving)))

(event Collision|EventActorBeginOverlap
  (params (OtherActor :type Actor%20Object%20Reference)))

(event EventTick
  (params (DeltaSeconds :type Float%20%28single-precision%29))
  (if (Variables|Default|GetShouldMove)
    (Variables|Default|SetDeltaTime DeltaSeconds)
    (if (Variables|Default|GetIsMoving)
      (CallFunction|Move (Variables|Default|GetCurrentDirection))
      (else
        (Variables|Default|SetMoveTimer (- (Variables|Default|GetMoveTimer) (Variables|Default|GetDeltaTime)))
        (if (<= (Variables|Default|GetMoveTimer) 0.0)
          (Variables|Default|SetIsMoving true)
          (Variables|Default|SetLocationToMoveFrom%20 (Transformation|GetActorLocation))
          (Development|PrintString "Hello")
          (bind (_moveup _movedown _moveright _moveleft) (CallFunction|CalculateMovement))
          (if _moveup
            (Utilities|Array|Add (Variables|Default|GetDirections) 0)
            (Development|PrintString "Up in array" true true "(R=0.000000,G=0.660000,B=1.000000,A=1.000000)" 1e+01))
          (if _movedown
            (Utilities|Array|Add (Variables|Default|GetDirections) 1)
            (Development|PrintString "Down in array" true true "(R=0.000000,G=0.660000,B=1.000000,A=1.000000)" 1e+01))
          (if _moveright
            (Utilities|Array|Add (Variables|Default|GetDirections) 2)
            (Development|PrintString "Right in array" true true "(R=0.000000,G=0.660000,B=1.000000,A=1.000000)" 1e+01))
          (if _moveleft
            (Utilities|Array|Add (Variables|Default|GetDirections) 3)
            (Development|PrintString "Left in array" true true "(R=0.000000,G=0.660000,B=1.000000,A=1.000000)" 1e+01))
          (if (> (Utilities|Array|Length (Variables|Default|GetDirections)) 0)
            (Variables|Default|SetCurrentDirection (.OutItem (Utilities|Array|Random (Variables|Default|GetDirections))))
            (else
              (Development|PrintString "Nowhere to move" true true "(R=0.000000,G=0.660000,B=1.000000,A=1.000000)" 1e+01))))))))

(fn ConstructionScript)

(fn Move
  (params (Direction :type Integer))
  (bind _locationtomovefrom_ (Variables|Default|GetLocationToMoveFrom%20))
  (bind _locationtomovefrom__2 (Variables|Default|GetLocationToMoveFrom%20))
  (bind _locationtomovefrom__3 (Variables|Default|GetLocationToMoveFrom%20))
  (bind _locationtomovefrom__4 (Variables|Default|GetLocationToMoveFrom%20))
  (switch int Direction
    (:0
      (Development|PrintString "Up selected" true true "(R=0.000000,G=0.660000,B=1.000000,A=1.000000)" 1e+01)
      (Transformation|SetActorLocation (Math|Interpolation|VInterpTo (Transformation|GetActorLocation) (Math|Vector|MakeVector (+ (.x _locationtomovefrom__3) (Variables|Default|GetMovementDistance)) (.y _locationtomovefrom__3) (.z _locationtomovefrom__3)) (Variables|Default|GetDeltaTime) 1e+01) false false))
    (:1
      (Development|PrintString "Down selected" true true "(R=0.000000,G=0.660000,B=1.000000,A=1.000000)" 1e+01)
      (Transformation|SetActorLocation (Math|Interpolation|VInterpTo (Transformation|GetActorLocation) (Math|Vector|MakeVector (- (.x _locationtomovefrom__4) (Variables|Default|GetMovementDistance)) (.y _locationtomovefrom__4) (.z _locationtomovefrom__4)) (Variables|Default|GetDeltaTime) 1e+01) false false))
    (:2
      (Development|PrintString "Right selected" true true "(R=0.000000,G=0.660000,B=1.000000,A=1.000000)" 1e+01)
      (Transformation|SetActorLocation (Math|Interpolation|VInterpTo (Transformation|GetActorLocation) (Math|Vector|MakeVector (.x _locationtomovefrom__2) (+ (.y _locationtomovefrom__2) (Variables|Default|GetMovementDistance)) (.z _locationtomovefrom__2)) (Variables|Default|GetDeltaTime) 1e+01) false false))
    (:3
      (Development|PrintString "Left selected" true true "(R=0.000000,G=0.660000,B=1.000000,A=1.000000)" 1e+01)
      (Transformation|SetActorLocation (Math|Interpolation|VInterpTo (Transformation|GetActorLocation) (Math|Vector|MakeVector (.x _locationtomovefrom_) (- (.y _locationtomovefrom_) (Variables|Default|GetMovementDistance)) (.z _locationtomovefrom_)) (Variables|Default|GetDeltaTime) 1e+01) false false))))

(fn SetMoveTimer
  (bind _output_get (Variables|Default|SetTimeBetweenMoving (Math|Random|RandomFloatinRange (Variables|Default|GetTimeBetweenMovingMin) (Variables|Default|GetTimeBetweenMovingMax))))
  (Development|PrintString (Utilities|String|ToString(Float) _output_get)))

(fn CalculateMovement
  (bind _returnvalue (Class|KismetSystemLibrary|SphereTraceSinglebyProfile (Variables|Default|GetLocationToMoveFrom%20) (+ (Variables|Default|GetLocationToMoveFrom%20) (Math|Vector|MakeVector (* (Variables|Default|GetMovementDistance) -1.0) 0.0 0.0)) 3e+01 "KeyboardKey" false 0 "Persistent" true))
  (if _returnvalue
    (Development|PrintString "Can't move down")
    (LocalVariables|SetCanMoveDown false))
  (bind _returnvalue_2 (Class|KismetSystemLibrary|SphereTraceSinglebyProfile (Variables|Default|GetLocationToMoveFrom%20) (+ (Variables|Default|GetLocationToMoveFrom%20) (Math|Vector|MakeVector (Variables|Default|GetMovementDistance) 0.0 0.0)) 3e+01 "KeyboardKey" false 0 "Persistent" true))
  (if _returnvalue_2
    (Development|PrintString "Can't move up")
    (LocalVariables|SetCanMoveUp false))
  (bind _returnvalue_3 (Class|KismetSystemLibrary|SphereTraceSinglebyProfile (Variables|Default|GetLocationToMoveFrom%20) (+ (Variables|Default|GetLocationToMoveFrom%20) (Math|Vector|MakeVector 0.0 (Variables|Default|GetMovementDistance) 0.0)) 3e+01 "KeyboardKey" false 0 "Persistent" true))
  (if _returnvalue_3
    (Development|PrintString "Can't move right")
    (LocalVariables|SetCanMoveRight false))
  (bind _returnvalue_4 (Class|KismetSystemLibrary|SphereTraceSinglebyProfile (Variables|Default|GetLocationToMoveFrom%20) (+ (Variables|Default|GetLocationToMoveFrom%20) (Math|Vector|MakeVector 0.0 (* (Variables|Default|GetMovementDistance) -1.0) 0.0)) 3e+01 "KeyboardKey" false 0 "Persistent" true))
  (if _returnvalue_4
    (Development|PrintString "Can't move left")
    (LocalVariables|SetCanMoveLeft false))
  (return (LocalVariables|GetCanMoveUp) (LocalVariables|GetCanMoveDown) (LocalVariables|GetCanMoveRight) (LocalVariables|GetCanMoveLeft)))